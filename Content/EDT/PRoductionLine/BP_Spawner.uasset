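; Production line spawner that periodically creates Item actors while its Interact flag is true.
; On BeginPlay it caches the GoToHere location as InteractPosition.
; Tick runs a timer that spawns at SpawnPoint with random yaw and 100x its scale, then passes RollingCarpet to the new BP_Item.
; It also pulses the actor's scale up to 1.1, finishing the pulse back at normal size after Interact turns off.
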(event `self.ReceiveBeginPlay`
  (set `self.InteractPosition` (`SceneComponent.K2_GetComponentLocation` (`self.GoToHere`))))

(event `self.ReceiveTick`
  (params (DeltaSeconds :type "Float (single-precision)"))
  (if (`self.bInteract`)
    (`self.SpawnItem` DeltaSeconds)
    (`self.AnimationScale` DeltaSeconds :!label _label)
    (elif (> (`self.Time Animation`) 0.0)
      (goto _label)
      (elif (`self.Up Down`)
        (goto _label)))))

(fn `AnimationScale`
  (params (A :type "Float (double-precision)"))
  (bind _returnvalue (+ A (`self.Time Animation`)))
  (if (`self.Up Down`)
    (`self.SetActorScale3D` (`KismetMathLibrary.VLerp` (1.1 1.1 1.1) (1.0 1.0 1.0) _returnvalue))
    (else
      (`self.SetActorScale3D` (`KismetMathLibrary.VLerp` (1.0 1.0 1.0) (1.1 1.1 1.1) _returnvalue))))
  (bind _output_get (set `self.Time Animation` _returnvalue))
  (if (>= _output_get 1.0)
    (if (`self.Up Down`)
      (set `self.Up Down` false)
      (else
        (set `self.Up Down` true)))
    (set `self.Time Animation` 0.0)))

(fn `SpawnItem`
  (params (A :type "Float (double-precision)"))
  (bind (_returnvalue_roll _returnvalue_pitch _returnvalue_yaw) (`KismetMathLibrary.BreakRotator` (`KismetMathLibrary.RandomRotator` true)))
  (bind _returnvalue (`SceneComponent.K2_GetComponentToWorld` (`self.SpawnPoint`)))
  (bind _output_get (set `self.Time` (+ A (`self.Time`))))
  (if (>= _output_get (`self.Timer`))
    (set `self.Time` 0.0)
    (bind _returnvalue_2 (`|SpawnActorFromClass` (`self.Item`) (`KismetMathLibrary.MakeTransform` (.location _returnvalue) (`KismetMathLibrary.MakeRotator` (.roll (.rotation _returnvalue)) (.pitch (.rotation _returnvalue)) _returnvalue_yaw) (* (.scale _returnvalue) (100.0 100.0 100.0))) "Undefined" "OverrideRootScale" null null))
    (bind _asbp_item (cast `/Game/EDT/PRoductionLine/BP_Item` _returnvalue_2))
    (set `/Game/EDT/PRoductionLine/BP_Item.RollingCarpet` (`self.RollingCarpet`) _asbp_item)))

(fn `UserConstructionScript`)