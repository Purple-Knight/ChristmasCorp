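; BP_RollingCarpetManual is a manually operated rolling carpet for a production line, built on a parent Blueprint.
; On BeginPlay it runs the parent logic and caches the world location of its GoToHere component as InteractPosition.
; While Interact is true, Tick accumulates delta time and sets ItemGo each time a second has elapsed, then resets the timer.
; Nothing in this graph sets Interact or clears ItemGo.
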(event `self.ReceiveBeginPlay`
  (`parent.ReceiveBeginPlay`)
  (set `self.InteractPosition` (`SceneComponent.K2_GetComponentLocation` (`self.GoToHere`))))

(event `self.ReceiveTick`
  (params (DeltaSeconds :type "Float (single-precision)"))
  (if (`self.bInteract`)
    (bind _output_get (set `self.Time` (+ DeltaSeconds (`self.Time`))))
    (if (>= _output_get 1.0)
      (set `self.ItemGo` true)
      (set `self.Time` 0.0))))

(fn `UserConstructionScript`
  (`parent.UserConstructionScript`))