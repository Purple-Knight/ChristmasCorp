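; Production-line machine that swallows BP_Items entering its box and, while interacted with, periodically spawns output items onto the next rolling carpet.
; The stored count over max stack forms an overload ratio driving the progress bar, loop pitch and volume, shaking and alarm.
; An item arriving at a full machine triggers explosions, ejecting items at the drop point and emptying the stack.
; Use also plays smoke puffs and a Tick-driven scale pulse.
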(event `self.ReceiveBeginPlay`
  (set `self.InteractPosition` (`SceneComponent.K2_GetComponentLocation` (`self.GoToHere`)))
  ;[1 1 1] Audio Machine
  (bind _returnvalue (`GameplayStatics.SpawnSoundAtLocation` (`self.LoopSound`) (`self.K2_GetActorLocation`) (struct) 1.0 1.0 0.0 null null))
  (bind _output_get (set `self.Audio_LoopMachine` _returnvalue))
  (`AudioComponent.Play` _output_get 0.0)
  (if (== (`self.MaxItemStack`) 0)
    (`SceneComponent.SetVisibility` (`self.BlackExplo`) false false)
    (else
      (`PaperFlipbookComponent.SetPlaybackPosition` (`self.WhiteSmoke1`) 9.0 false)
      (`PaperFlipbookComponent.SetPlaybackPosition` (`self.WhiteSmoke`) 9.0 false)
      (`PaperFlipbookComponent.SetPlaybackPosition` (`self.WhiteSmoke2`) 9.0 false)
      (`PaperFlipbookComponent.SetPlaybackPosition` (`self.WhiteSmoke3`) 9.0 false)
      (`PaperFlipbookComponent.SetPlaybackPosition` (`self.BlackExplo`) 9.0 false)
      (`SceneComponent.SetVisibility` (`self.BlackExplo`) false false))))

(event `self.ReceiveTick`
  (params (DeltaSeconds :type "Float (single-precision)"))
  (bind _whitesmoke (`self.WhiteSmoke`))
  (bind _whitesmoke1 (`self.WhiteSmoke1`))
  (bind _whitesmoke2 (`self.WhiteSmoke2`))
  (bind _whitesmoke3 (`self.WhiteSmoke3`))
  (`|ExecutionSequence`
    (:`then_0`
      (`self.SetOverLoad`)
      (if (`self.bInteract`)
        (`|ExecutionSequence`
          (:`then_0`
            (`self.SpawnItem` DeltaSeconds)
            ;[1 0.02901 0.1789] AUDIO USEmachine
            (`self.AnimationScale` DeltaSeconds :!label _label)
            (if (not (`self.bInteract`))
              (goto _label_2 :!via `Reset`)))
          (:`then_1`
            (`/Engine/EditorBlueprintResources/StandardMacros.DoOnce` false :!label _label_2
              (:`Completed`
                (`KismetSystemLibrary.Delay` 0.2)
                (`GameplayStatics.PlaySoundAtLocation` "/Game/EDT/SD/FACTORY_-_LD/FTR_I_UseMachine_01_Cue.FTR_I_UseMachine_01_Cue" (`self.K2_GetActorLocation`) (struct) 1.0 1.0 0.0 null null null null)
                (`PaperFlipbookComponent.SetPlaybackPosition` (`self.WhiteSmoke`) 0.0 false)
                (`PaperFlipbookComponent.SetPlaybackPosition` (`self.WhiteSmoke1`) 0.0 false)
                (`PaperFlipbookComponent.SetPlaybackPosition` (`self.WhiteSmoke2`) 0.0 false)
                (`PaperFlipbookComponent.SetPlaybackPosition` (`self.WhiteSmoke3`) 0.0 false)
                (`PaperFlipbookComponent.Play` (`self.WhiteSmoke`))
                (`PaperFlipbookComponent.Play` (`self.WhiteSmoke1`))
                (`PaperFlipbookComponent.Play` (`self.WhiteSmoke2`))
                (`PaperFlipbookComponent.Play` (`self.WhiteSmoke3`))
                (`KismetSystemLibrary.Delay` 0.8)
                (`PaperFlipbookComponent.SetPlaybackPosition` _whitesmoke 9.0 false)
                (`PaperFlipbookComponent.Stop` _whitesmoke)
                (`PaperFlipbookComponent.SetPlaybackPosition` _whitesmoke1 9.0 false)
                (`PaperFlipbookComponent.Stop` _whitesmoke1)
                (`PaperFlipbookComponent.SetPlaybackPosition` _whitesmoke2 9.0 false)
                (`PaperFlipbookComponent.Stop` _whitesmoke2)
                (`PaperFlipbookComponent.SetPlaybackPosition` _whitesmoke3 9.0 false)
                (`PaperFlipbookComponent.Stop` _whitesmoke3)))))
        (elif (> (`self.TimeAnimation`) 0.0)
          (goto _label)
          (elif (`self.UpDown`)
            (goto _label)))))
    (:`then_1`
      ;[1 1 1] Set Audio Pitch Machine
      (`AudioComponent.SetPitchMultiplier` (`self.Audio_LoopMachine`) (`KismetMathLibrary.MapRangeClamped` (`self.Pourcentage`) 0.0 1.0 1.0 2.0))
      (`AudioComponent.SetVolumeMultiplier` (`self.Audio_LoopMachine`) (`KismetMathLibrary.MapRangeClamped` (`self.Pourcentage`) 0.0 1.0 0.75 2.0))
      (if (>= (`self.Pourcentage`) 0.8)
        (`|ExecutionSequence`
          (:`then_0`
            (`/Engine/EditorBlueprintResources/StandardMacros.DoOnce` false :!label _label_3
              (:`Completed`
                (bind _returnvalue (`GameplayStatics.SpawnSoundAtLocation` "/Game/EDT/SD/FACTORY_-_LD/FTR_Alarm_Cue.FTR_Alarm_Cue" (`self.K2_GetActorLocation`) (struct) 1.0 1.0 0.0 null null))
                (`AudioComponent.Play` _returnvalue 0.0))))
          (:`then_1`
            (goto _label_4 :!via `Reset`)))
        (else
          (`|ExecutionSequence`
            (:`then_0`
              (goto _label_3 :!via `Reset`))
            (:`then_1`
              (`/Engine/EditorBlueprintResources/StandardMacros.DoOnce` true :!label _label_4
                (:`Completed`
                  (`AudioComponent.Stop` _returnvalue))))))))))

(event `self.Box.OnComponentBeginOverlap`
  (params (OverlappedComponent :type "PrimitiveComponent Object Reference") (OtherActor :type "Actor Object Reference") (OtherComp :type "PrimitiveComponent Object Reference") (OtherBodyIndex :type Integer) (bFromSweep :type Boolean) (SweepResult :type "HitResult Structure (by ref)"))
  (bind _itementer (`self.ItemEnter`))
  (bind _blackexplo (`self.BlackExplo`))
  (bind _blackexplo_2 (`self.BlackExplo`))
  (bind _returnvalue (`SceneComponent.K2_GetComponentLocation` (`self.DropPoint`)))
  (bind _asbp_item (cast `/Game/EDT/PRoductionLine/BP_Item` OtherActor))
  (if (>= _itementer (`self.MaxItemStack`))
    (set `/Game/EDT/PRoductionLine/BP_Item.RollingCarpet` null _asbp_item)
    (`SceneComponent.K2_SetWorldLocation` (`/Game/EDT/PRoductionLine/BP_Item.Cube` _asbp_item) _returnvalue false true)
    (set `/Game/EDT/PRoductionLine/BP_Item.Eject` true _asbp_item)
    (for _ (range (+ (`self.ItemEnter`) 1))
      (bind _returnvalue_2 (`|SpawnActorFromClass` (`GameplayStatics.GetObjectClass` _asbp_item) (`KismetMathLibrary.MakeTransform` _returnvalue) "Undefined" "MultiplyWithRoot" null null))
      (set `/Game/EDT/PRoductionLine/BP_Item.Eject` true _returnvalue_2)
      (`GameplayStatics.PlaySoundAtLocation` "/Game/StarterContent/Audio/Explosion_Cue.Explosion_Cue" (`self.K2_GetActorLocation`) (struct) 1.0 1.0 0.0 null null null null)
      (`PaperFlipbookComponent.SetPlaybackPosition` _blackexplo_2 0.0 false)
      (`SceneComponent.SetVisibility` (`self.BlackExplo`) true false)
      (`PaperFlipbookComponent.Play` _blackexplo_2)
      (`KismetSystemLibrary.Delay` 0.8)
      (`PaperFlipbookComponent.SetPlaybackPosition` _blackexplo 9.0 false)
      (`PaperFlipbookComponent.Stop` _blackexplo)
      (`SceneComponent.SetVisibility` (`self.BlackExplo`) false false))
    (set `self.ItemEnter` 0)
    (else
      (`/Engine/EditorBlueprintResources/StandardMacros.IncrementInt` _itementer
        (:`  `
          (`self.K2_DestroyActor` _asbp_item)
          (`self.SetOverLoad`))))))

(fn `AnimationScale`
  (params (A :type "Float (double-precision)"))
  (bind _returnvalue (+ A (`self.TimeAnimation`)))
  (if (`self.UpDown`)
    (`self.SetActorScale3D` (`KismetMathLibrary.VLerp` (1.1 1.1 1.1) (1.0 1.0 1.0) _returnvalue))
    (else
      (`self.SetActorScale3D` (`KismetMathLibrary.VLerp` (1.0 1.0 1.0) (1.1 1.1 1.1) _returnvalue))))
  (set `self.TimeAnimation` _returnvalue)
  (if (>= (`self.TimeAnimation`) 1.0)
    (if (`self.UpDown`)
      (set `self.UpDown` false)
      (else
        (set `self.UpDown` true)))
    (set `self.TimeAnimation` 0.0)))

(fn `SetOverLoad`
  (bind _widget (`self.Widget`))
  (bind _pourcentage (`self.Pourcentage`))
  (bind _pourcentage_2 (`self.Pourcentage`))
  (bind _machine (`self.machine`))
  (bind (_returnvalue_roll _returnvalue_pitch _returnvalue_yaw) (`KismetMathLibrary.BreakRotator` (`SceneComponent.K2_GetComponentRotation` _machine)))
  (bind _returnvalue (+ _returnvalue_roll _pourcentage))
  (bind _returnvalue_2 (- _returnvalue_pitch _pourcentage))
  (`|ExecutionSequence`
    (:`then_0`
      ;[1 0.02061 0.04051] Pourcentage audio
      (bind _output_get (set `self.Pourcentage` (/ (`KismetMathLibrary.Conv_IntToDouble` (`self.ItemEnter`)) (`KismetMathLibrary.Conv_IntToDouble` (`self.MaxItemStack`)))))
      (if (>= _output_get 0.75)
        (if (`self.LeftRight`)
          (`SceneComponent.K2_SetWorldRotation` _machine (`KismetMathLibrary.MakeRotator` _returnvalue _returnvalue_2 _returnvalue_yaw) false false)
          (set `self.LeftRight` false)
          (else
            (`SceneComponent.K2_SetWorldRotation` _machine (`KismetMathLibrary.MakeRotator` _returnvalue_2 _returnvalue _returnvalue_yaw) false false)
            (set `self.LeftRight` true)))))
    (:`then_1`
      (bind _aswb_over_load_progresse_bar (cast `/Game/EDT/PRoductionLine/WB_OverLoadProgresseBar` (`WidgetComponent.GetUserWidgetObject` _widget)))
      (`ProgressBar.SetPercent` (`/Game/EDT/PRoductionLine/WB_OverLoadProgresseBar.ProgressBar_41` _aswb_over_load_progresse_bar) _pourcentage_2)
      (if (or (== _pourcentage_2 1.0) (== _pourcentage_2 0.0))
        (`SceneComponent.SetVisibility` _widget false false)
        (else
          (`SceneComponent.SetVisibility` _widget true false))))))

(fn `SpawnItem`
  (params (A :type "Float (double-precision)"))
  (bind (_returnvalue_roll _returnvalue_pitch _returnvalue_yaw) (`KismetMathLibrary.BreakRotator` (`KismetMathLibrary.RandomRotator` true)))
  (bind _output_get (set `self.Time` (+ A (`self.Time`))))
  (if (>= _output_get (`self.Timer`))
    (if (> (`self.ItemEnter`) 0)
      (set `self.ItemEnter` (- (`self.ItemEnter`) 1))
      (bind _returnvalue (`|SpawnActorFromClass` (`self.Object`) (`KismetMathLibrary.MakeTransform` (.location (`SceneComponent.K2_GetComponentToWorld` (`/Game/EDT/PRoductionLine/BP_RollingCarpet.StartPoint` (`self.NextRollingCarpet`)))) (`KismetMathLibrary.MakeRotator` 0.0 0.0 _returnvalue_yaw)) "Undefined" "OverrideRootScale" null null))
      (bind _asbp_item (cast `/Game/EDT/PRoductionLine/BP_Item` _returnvalue))
      (set `/Game/EDT/PRoductionLine/BP_Item.RollingCarpet` (`self.NextRollingCarpet`) _asbp_item)
      ;[0 1 0.7556] Audio
      (`GameplayStatics.PlaySoundAtLocation` (`self.SpawnSound`) (`SceneComponent.K2_GetComponentLocation` (`self.machine`)) (struct) 1.0 1.0 0.0 null null null null))
    (set `self.Time` 0.0)))

(fn `UserConstructionScript`)