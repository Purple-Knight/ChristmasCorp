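; BP_Item is a production-line item that plays a spawn sound and rides along chained rolling carpets.
; Tick lerps it between each carpet's start and end points, then hands it to the next carpet or enables physics.
; Manual carpets queue items, releasing the first on ItemGo and moving items only while Interact is true.
; Setting Eject launches the cube randomly with physics and destroys the actor after a delay.
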(event `self.ReceiveTick`
  (params (DeltaSeconds :type "Float (single-precision)"))
  (bind _returnvalue (`KismetMathLibrary.RandomUnitVector`))
  (bind _rollingcarpet (`self.RollingCarpet`))
  (bind _cube (`self.Cube`))
  (bind _next (`/Game/EDT/PRoductionLine/BP_RollingCarpet.Next` (`self.RollingCarpet`)))
  (bind _returnvalue_2 (+ (* (/ DeltaSeconds 100.0) (`self.Speed`)) (`self.Time`)))
  (if (`self.Eject`)
    (`PrimitiveComponent.SetSimulatePhysics` (`self.Cube`) true)
    (`PrimitiveComponent.SetPhysicsLinearVelocity` _cube (+ (0.0 0.0 400.0) (* _returnvalue (500.0 500.0 1.0))) false "None")
    (`PrimitiveComponent.AddVelocityChangeImpulseAtLocation` _cube _returnvalue (0.0 0.0 0.0) "None")
    (`SceneComponent.K2_SetWorldRotation` _cube (`KismetMathLibrary.RandomRotator` true) false false)
    (set `self.Eject` false)
    (`KismetSystemLibrary.Delay` 10.0)
    (`self.K2_DestroyActor`)
    (elif (< (`self.Time`) 1.0)
      (bind _asbp_rolling_carpet_manual (cast `/Game/EDT/PRoductionLine/BP_RollingCarpetManual` (`self.RollingCarpet`))
        (:`then`
          (if (`Interactable.bInteract` _asbp_rolling_carpet_manual)
            (if (!= (`self.Time`) 0.0)
              (`SceneComponent.K2_SetWorldLocation` (`self.DefaultSceneRoot`) (`KismetMathLibrary.VLerp` (`SceneComponent.K2_GetComponentLocation` (`/Game/EDT/PRoductionLine/BP_RollingCarpet.StartPoint` _rollingcarpet)) (`SceneComponent.K2_GetComponentLocation` (`/Game/EDT/PRoductionLine/BP_RollingCarpet.EndPoint` _rollingcarpet)) _returnvalue_2) false false :!label _label)
              (set `self.Time` _returnvalue_2)
              (elif (`/Game/EDT/PRoductionLine/BP_RollingCarpetManual.ItemGo` _asbp_rolling_carpet_manual)
                (bind _item (`/Game/EDT/PRoductionLine/BP_RollingCarpetManual.Item` _asbp_rolling_carpet_manual))
                (if (== (`|GetArrayItem` _item) self)
                  (set `/Game/EDT/PRoductionLine/BP_RollingCarpetManual.ItemGo` false _asbp_rolling_carpet_manual)
                  (`KismetSystemLibrary.Delay` 0.1)
                  (`KismetArrayLibrary.Array_Remove` _item)
                  (goto _label))))))
        (:`CastFailed`
          (cast `/Game/EDT/PRoductionLine/BP_RollingCarpet` (`self.RollingCarpet`))
          (goto _label)))
      (else
        ;[1 1 1] Check For Change Rolling Carpet
        (if (!= _next "/Game/EDT/PRoductionLine/BP_RollingCarpet.BP_RollingCarpet")
          (bind _output_get (set `self.RollingCarpet` _next))
          (bind _asbp_rolling_carpet_manual_2 (cast `/Game/EDT/PRoductionLine/BP_RollingCarpetManual` _output_get)
            (:`then`
              (`KismetArrayLibrary.Array_Add` (`/Game/EDT/PRoductionLine/BP_RollingCarpetManual.Item` _asbp_rolling_carpet_manual_2) self))
            (:`CastFailed`
              _))
          (else
            (`PrimitiveComponent.SetSimulatePhysics` (`self.Cube`) true)))
        (set `self.Time` 0.0)))))

(event `self.ReceiveBeginPlay`
  ;[1 0 0] Audio Spawn item
  (`GameplayStatics.PlaySoundAtLocation` "/Game/EDT/SD/FACTORY_-_LD/FTR_G_Spawn_Cue.FTR_G_Spawn_Cue" (`self.K2_GetActorLocation`) (struct) 1.0 1.0 0.0 null null null null))

(fn `UserConstructionScript`)