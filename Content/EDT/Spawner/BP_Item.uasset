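; BP_Item is an item that rides a chain of rolling carpets, moving from each carpet's start point to its end point.
; Tick advances a normalized Time by frame delta and Speed, then lerps the root's world location between the current carpet's StartPoint and EndPoint with sweep enabled.
; Once Time reaches one, it switches to the carpet's Next link and resets Time, or stops moving if there is none.
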(event `self.ReceiveTick`
  (params (DeltaSeconds :type "Float (single-precision)"))
  (bind _rollingcarpet (`self.RollingCarpet`))
  (bind _next (`/Game/EDT/Spawner/BP_RollingCarpet.Next` (`self.RollingCarpet`)))
  (bind _returnvalue (+ (* (/ DeltaSeconds 100.0) (`self.Speed`)) (`self.Time`)))
  (if (< (`self.Time`) 1.0)
    (set `self.Time` _returnvalue)
    (`SceneComponent.K2_SetWorldLocation` (`self.DefaultSceneRoot`) (`KismetMathLibrary.VLerp` (`SceneComponent.K2_GetComponentLocation` (`/Game/EDT/Spawner/BP_RollingCarpet.StartPoint` _rollingcarpet)) (`SceneComponent.K2_GetComponentLocation` (`/Game/EDT/Spawner/BP_RollingCarpet.EndPoint` _rollingcarpet)) _returnvalue) true false)
    (elif (!= _next null)
      (set `self.RollingCarpet` _next)
      (set `self.Time` 0.0))))

(fn `UserConstructionScript`)