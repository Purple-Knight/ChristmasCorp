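; BP_Spawner is an actor that repeatedly spawns items and links each one to a rolling carpet.
; Tick accumulates delta time and, on reaching the Timer interval, resets it and spawns the Item class at the SpawnPoint transform, multiplying its scale a hundredfold.
; Each spawned actor is cast to BP_Item and receives the spawner's RollingCarpet reference.
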(event `self.ReceiveTick`
  (params (DeltaSeconds :type "Float (single-precision)"))
  (bind (_returnvalue_location _returnvalue_rotation _returnvalue_scale) (`KismetMathLibrary.BreakTransform` (`SceneComponent.K2_GetComponentToWorld` (`self.SpawnPoint`))))
  (bind _output_get (set `self.Time` (+ DeltaSeconds (`self.Time`))))
  (if (>= _output_get (`self.Timer`))
    (set `self.Time` 0.0)
    (bind _returnvalue (`|SpawnActorFromClass` (`self.Item`) (`KismetMathLibrary.MakeTransform` _returnvalue_location _returnvalue_rotation (* _returnvalue_scale (100.0 100.0 100.0))) "Undefined" "OverrideRootScale" null null))
    (bind _asbp_item (cast `/Game/EDT/Spawner/BP_Item` _returnvalue))
    (set `/Game/EDT/Spawner/BP_Item.RollingCarpet` (`self.RollingCarpet`) _asbp_item)))

(fn `UserConstructionScript`)