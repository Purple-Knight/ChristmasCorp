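; BP_TimeManager is an actor that runs an in-game clock from a starting hour to an ending hour.
; BeginPlay sets the clock to the starting hour, and Tick uses a Delay of DurationOfMin to pace each minute increment.
; Minutes roll over into hours, which wrap to zero after 23.
; Once the ending hour is reached, the clock stops advancing and Tick prints a "Day Over!" message.
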(event `self.ReceiveBeginPlay`
  ;[1 1 1] When actor is added / enabled in the level, sets "Current Time" to "Starting Hour" indicated in inspector.
  (set `self.currentMinute` 0)
  (set `self.currentHour` (`self.startingHour`)))

(event `self.ReceiveTick`
  (params (DeltaSeconds :type "Float (single-precision)"))
  (bind _currentminute (`self.currentMinute`))
  ;[1 1 1] Check if day is over.
  (if (>= (`self.currentHour`) (`self.endingHour`))
    ;[1 1 1] If day is over do :
    (`KismetSystemLibrary.PrintString` "Day Over!")
    (else
      ;[1 1 1] If day isn't over, increases "Current Time" by "Duration Of Min" :
      (`KismetSystemLibrary.Delay` (`self.durationOfMin`))
      (set `self.currentMinute` (+ _currentminute 1))
      (if (> _currentminute 59)
        (if (> (`self.currentHour`) 22)
          (set `self.currentHour` 0)
          (set `self.currentMinute` 0)
          (else
            (set `self.currentMinute` 0)
            (set `self.currentHour` (+ (`self.currentHour`) 1))))))))

(fn `UserConstructionScript`)