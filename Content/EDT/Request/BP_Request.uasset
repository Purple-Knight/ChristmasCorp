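; BP_Request runs a timed item request with a star rating that drops as time passes.
; BeginPlay creates the request HUD and adds one text entry showing the item count.
; Once started, Tick advances the timer, clearing star flags and shifting its color toward red at successive thresholds.
; The request ends when the entry list empties or time passes the lose limit, calling CallEnd and fading the UI.
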(event `self.ReceiveBeginPlay`
  (bind _returnvalue (`|CreateWidget` "/Game/EDT/Request/WB_Request.WB_Request_C"))
  (`UserWidget.AddToViewport` _returnvalue 0)
  (bind _output_get (set `self.UI` _returnvalue))
  (bind _returnvalue_2 (`|CreateWidget` "/Game/EDT/Request/WB_TextRequest.WB_TextRequest_C"))
  (`KismetArrayLibrary.Array_Add` (`self.TextRequest`) _returnvalue_2)
  (set `TextBlock.Text` (`KismetTextLibrary.Conv_IntToText` (`self.ItemCont`)) (`/Game/EDT/Request/WB_TextRequest.Count` _returnvalue_2))
  (`PanelWidget.AddChild` (`/Game/EDT/Request/WB_Request.HorizontalBox_0` _output_get) _returnvalue_2)
  (`UserWidget.SetPadding` _returnvalue_2 (make `Margin` 20.0 20.0 20.0 20.0)))

(event `self.ReceiveTick`
  (params (DeltaSeconds :type "Float (single-precision)"))
  (`|ExecutionSequence`
    (:`then_0`
      (if (<= (`KismetArrayLibrary.Array_Length` (`self.TextRequest`)) 0)
        (`/Engine/EditorBlueprintResources/StandardMacros.DoOnce` false
          (:`Completed`
            (`self.CallEnd`)
            (set `self.isFinished` true)
            (`/Game/EDT/Request/WB_Request.FadeUI` (`self.UI`))))))
    (:`then_1`
      (if (not (`self.isFinished`))
        (`self.TimerFonction` DeltaSeconds)))))

(fn `TimerFonction`
  (params (B :type "Float (double-precision)"))
  (bind _returnvalue (+ B (`self.Time`)))
  (bind _timer (`/Game/EDT/Request/WB_Request.Timer` (`self.UI`)))
  (if (`self.Start`)
    (set `TextBlock.Text` (`KismetTextLibrary.Conv_StringToText` (`KismetStringLibrary.LeftChop` (`KismetStringLibrary.TimeSecondsToString` _returnvalue) 3)) _timer)
    (bind _output_get (set `self.Time` _returnvalue))
    (if (< (`self.3Stars`) _output_get)
      (`|ExecutionSequence`
        (:`then_0`
          (set `self.isStar3` false))
        (:`then_1`
          (set `TextBlock.ColorAndOpacity` (make `SlateColor` (struct :`R` 1.0 :`G` 0.926 :`A` 1.0)) _timer)
          (if (< (`self.2Stars`) _output_get)
            (`|ExecutionSequence`
              (:`then_0`
                (set `self.isStar2` false))
              (:`then_1`
                (set `TextBlock.ColorAndOpacity` (make `SlateColor` (struct :`R` 1.0 :`G` 0.367 :`A` 1.0)) _timer)
                (if (< (`self.1Stars`) _output_get)
                  (`|ExecutionSequence`
                    (:`then_0`
                      (set `self.isStar1` false))
                    (:`then_1`
                      (set `TextBlock.ColorAndOpacity` (make `SlateColor` (struct :`R` 1.0 :`A` 1.0)) _timer)
                      (if (< (`self.Loose`) _output_get)
                        (`/Engine/EditorBlueprintResources/StandardMacros.DoOnce` false
                          (:`Completed`
                            (if (not (`self.isFinished`))
                              (`self.CallEnd`)
                              (set `self.isFinished` true)
                              (`/Game/EDT/Request/WB_Request.FadeUI` (`self.UI`)))))))))))))))))

(fn `UserConstructionScript`)